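; Actor that moves its Sphere component along its Spline, starting from the spline's beginning.
; Tick adds Speed to Distance each frame without delta-time scaling or wrapping, then places the Sphere at that distance.
; The Sphere's rotation comes from looking at a point slightly further along the spline.
; Disconnected nodes for cursor-based sphere spawning and spline point adding never run.
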(event EventBeginPlay
  (bind _spline (Variables|Default|GetSpline))
  (Variables|Default|Setdistance 0.0)
  (Transformation|SetWorldLocationAndRotation (Variables|Default|GetSphere) (Spline|GetLocationatDistanceAlongSpline _spline (Variables|Default|Getdistance) "World") (Math|Rotator|FindLookatRotation (Spline|GetLocationatDistanceAlongSpline _spline (Variables|Default|Getdistance) "World") (Spline|GetLocationatDistanceAlongSpline _spline (+ (Variables|Default|Getdistance) 5.0) "World")) false false))

(event Collision|EventActorBeginOverlap
  (params (OtherActor :type Actor%20Object%20Reference)))

(event EventTick
  (params (DeltaSeconds :type Float%20%28single-precision%29))
  (bind _spline (Variables|Default|GetSpline))
  (Variables|Default|Setdistance (+ (Variables|Default|Getspeed) (Variables|Default|Getdistance)))
  (Transformation|SetWorldLocationAndRotation (Variables|Default|GetSphere) (Spline|GetLocationatDistanceAlongSpline _spline (Variables|Default|Getdistance) "World") (Math|Rotator|FindLookatRotation (Spline|GetLocationatDistanceAlongSpline _spline (Variables|Default|Getdistance) "World") (Spline|GetLocationatDistanceAlongSpline _spline (+ (Variables|Default|Getdistance) 5.0) "World")) false false))

(fn ConstructionScript)