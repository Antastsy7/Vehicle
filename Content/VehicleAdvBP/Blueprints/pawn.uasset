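; Pawn that lets the player draw a mouse path, which its Sphere follows on release.
; SpaceBar toggles a top-down camera state where dragging from the pawn records points, shown by a line widget and ghost sphere.
; Drawing drains a percent meter by ticks or distance, stopping when empty; it regenerates in Normal state and feeds the UI.
; A Tick-checked state machine starts playback, stepping through points with short delays and orienting from earlier points.
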(event EventBeginPlay
  (bind _returnvalue (UserInterface|CreateWidget "/Game/VehicleAdvBP/Blueprints/UI.UI_C"))
  (UserInterface|Viewport|AddtoViewport _returnvalue 0)
  (Variables|Default|Setui _returnvalue))

(event Collision|EventActorBeginOverlap
  (params (OtherActor :type Actor%20Object%20Reference)))

(event EventTick
  (params (DeltaSeconds :type Float%20%28single-precision%29))
  (Development|PrintString (Utilities|String|EnumtoString (Variables|Default|Getstate)))
  (Progress|SetPercent)
  (switch Utilities|FlowControl|Switch|SwitchonStates (Variables|Default|Getstate)
    (:NewEnumerator1
      (|DrawMousePos (.ReturnValue (Game|Player|GetMousePosition))))
    (:NewEnumerator5
      (Variables|Default|Setstate "NewEnumerator3")
      (|Trace
        (:output
          (Variables|Default|Setstate "NewEnumerator0"))))))

(event Input|KeyboardEvents|SpaceBar
  (params (Key :type Key%20Structure))
  (bind _returnvalue (Game|GetPlayerController 0))
  (bind _camera (Variables|Default|GetCamera))
  (bind _camera_2 (Variables|Default|GetCamera))
  (:Pressed
    (Utilities|FlowControl|FlipFlop
      (:A
        (Variables|Default|Setstate "NewEnumerator0")
        (Game|SetGamePaused false)
        (Variables|/Script/Engine.PlayerController|SetbShowMouseCursor _returnvalue true)
        (Transformation|SetRelativeLocation _camera_2 "0, 0,2000.000000" false false)
        (Transformation|SetRelativeRotation _camera_2 "-90.000000, 0,-0.000000" false false))
      (:B
        (Variables|Default|Setstate "NewEnumerator4")
        (Game|SetGamePaused false)
        (Variables|/Script/Engine.PlayerController|SetbShowMouseCursor _returnvalue false)
        (Transformation|SetRelativeLocation _camera "-500.000000,0.000000,0.000000" false false)
        (Transformation|SetRelativeRotation _camera "0, 0, 0" false false)))))

(event Input|KeyboardEvents|1
  (params (Key :type Key%20Structure))
  (bind _returnvalue (Game|GetPlayerController 0))
  ;[1 1 1] show mouse
  (:Pressed
    (Variables|/Script/Engine.PlayerController|SetbShowMouseCursor _returnvalue true))
  (:Released
    (Variables|/Script/Engine.PlayerController|SetbShowMouseCursor _returnvalue false)))

(event Input|MouseEvents|LeftMouseButton
  (params (Key :type Key%20Structure))
  (:Pressed
    (switch Utilities|FlowControl|Switch|SwitchonStates (Variables|Default|Getstate)
      (:NewEnumerator0
        (if (== (.HitActor (Collision|BreakHitResult (.HitResult (Game|Player|GetHitResultUnderCursorbyChannel (Game|GetPlayerController 0) "TraceTypeQuery1" true)))) self)
          (Variables|Default|Setstate "NewEnumerator1")
          (|DrawTrace)))))
  (:Released
    (switch Utilities|FlowControl|Switch|SwitchonStates (Variables|Default|Getstate)
      (:NewEnumerator1
        _)
      (:NewEnumerator2
        _))
    (|ClearTrace)))

(fn ConstructionScript)

(fn DefaultArrays
  (bind _vectors (Variables|Default|GetVectors))
  (Utilities|Array|Clear (Variables|Default|GetTraces))
  (Utilities|Array|Clear _vectors)
  (Utilities|Array|Add _vectors (.ScreenPosition (Class|WidgetLayoutLibrary|ProjectWorldLocationtoWidgetPosition (Game|GetPlayerController 0) (Transformation|GetWorldLocation (Variables|Default|GetSphere))))))